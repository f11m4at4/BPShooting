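; BP_Enemy is an enemy actor that moves in a straight line, either downward or toward where the player was at spawn.
; BeginPlay finds BP_Player and randomly, at roughly even odds, sets Direction straight down or normalized toward the player.
; Tick moves the actor along that fixed Direction by Speed and delta time, without sweeping.
; Unconnected leftover nodes hold earlier variants, including continuous player homing.
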(event EventBeginPlay
  ;[1 1 1] 50% 미만인지 검사
  (bind _returnvalue (Actor|GetActorOfClass "/Game/Blueprints/BP_Player.BP_Player_C"))
  (Variables|Default|SetTarget _returnvalue)
  (if (< (Math|Random|RandomIntegerinRange 1 100) 50)
    ;[1 1 1] 방향을 구한다.
    (Variables|Default|SetDirection "0, 0,-1.000000")
    (else
      (Variables|Default|SetDirection (Math|Vector|Normalize (- (Transformation|GetActorLocation (Variables|Default|GetTarget)) (Transformation|GetActorLocation)))))))

(event EventTick
  (params (DeltaSeconds :type Float%20%28single-precision%29))
  ;[1 1 1] 이동한다.
  ;;[1 1 1] t
  ;;[1 1 1] P
  (Transformation|SetActorLocation (+ (Transformation|GetActorLocation) (* (* (Variables|Default|GetDirection) (Variables|Default|GetSpeed)) DeltaSeconds)) false false))

(fn ConstructionScript)